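; BP_Walls builds visual-only wall segments from a JSON file in the project directory.
; When IsVisible is set, the Construction Script loads Filename and reads each field as a pair of 3D points.
; Each pair becomes a static mesh component placed at the second point, aimed at the first and X-scaled by their distance over 100.
; Segments have collision disabled, and the event graph is empty.
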(event EventBeginPlay)

(event Collision|EventActorBeginOverlap
  (params (OtherActor :type Actor%20Object%20Reference)))

(event EventTick
  (params (DeltaSeconds :type Float%20%28single-precision%29)))

(fn ConstructionScript
  (if (Variables|Default|GetisVisible)
    (bind _outjsonobject (Class|JsonBlueprintFunctionLibrary|FromFile (Utilities|Struct|MakeFilePath (Class|KismetSystemLibrary|NormalizeFilename (Utilities|String|Append (Class|KismetSystemLibrary|GetProjectDirectory) (Variables|Default|Getfilename))))))
    (bind _fieldnames (Class|JsonBlueprintFunctionLibrary|GetFieldNames _outjsonobject))
    (for _array_element _fieldnames
      (bind _outvalue (|GetJsonField _outjsonobject _array_element))
      (bind _output_get (Variables|Default|SetWall%20Points _outvalue))
      (bind _returnvalue (AddComponent|AddStaticMeshComponent false (Math|Transform|MakeTransform (Math|Vector|MakeVector (Utilities|Array|Get(acopy) (.second (Utilities|Struct|BreakWallPoints _output_get))) (Utilities|Array|Get(acopy) (.second (Utilities|Struct|BreakWallPoints _output_get)) 1) (Utilities|Array|Get(acopy) (.second (Utilities|Struct|BreakWallPoints _output_get)) 2)) (Math|Conversions|RotationFromXVector (- (Math|Vector|MakeVector (Utilities|Array|Get(acopy) (.first (Utilities|Struct|BreakWallPoints _output_get))) (Utilities|Array|Get(acopy) (.first (Utilities|Struct|BreakWallPoints _output_get)) 1) (Utilities|Array|Get(acopy) (.first (Utilities|Struct|BreakWallPoints _output_get)) 2)) (Math|Vector|MakeVector (Utilities|Array|Get(acopy) (.second (Utilities|Struct|BreakWallPoints _output_get))) (Utilities|Array|Get(acopy) (.second (Utilities|Struct|BreakWallPoints _output_get)) 1) (Utilities|Array|Get(acopy) (.second (Utilities|Struct|BreakWallPoints _output_get)) 2)))) (Math|Vector|MakeVector (* (Math|Vector|VectorLength (- (Math|Vector|MakeVector (Utilities|Array|Get(acopy) (.first (Utilities|Struct|BreakWallPoints _output_get))) (Utilities|Array|Get(acopy) (.first (Utilities|Struct|BreakWallPoints _output_get)) 1) (Utilities|Array|Get(acopy) (.first (Utilities|Struct|BreakWallPoints _output_get)) 2)) (Math|Vector|MakeVector (Utilities|Array|Get(acopy) (.second (Utilities|Struct|BreakWallPoints _output_get))) (Utilities|Array|Get(acopy) (.second (Utilities|Struct|BreakWallPoints _output_get)) 1) (Utilities|Array|Get(acopy) (.second (Utilities|Struct|BreakWallPoints _output_get)) 2)))) 0.01) 1.0 1.0))))
      (Collision|SetCollisionEnabled _returnvalue "NoCollision"))))